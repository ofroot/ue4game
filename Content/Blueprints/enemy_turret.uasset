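; Enemy turret that turns to face the player character on sight and fires impulse-launched projectiles on a one-second cooldown.
; PawnSensing drives aiming and shooting, with a flag and delay gating the fire rate.
; Damage lowers health until death triggers explosion effects, radius damage on the SphereDm component and delayed destruction.
; Collision hits against another enemy_turret apply damage to that turret.
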(event `self.PawnSensing.OnSeePawn`
  (params (Pawn :type "Pawn Object Reference"))
  (if (`self.IsAlive`)
    (bind _asfirst_person_character (cast `/Game/FirstPersonBP/Blueprints/FirstPersonCharacter` Pawn))
    (`|ExecutionSequence`
      (:`then_0`
        (`self.K2_SetActorRotation` (`KismetMathLibrary.FindLookAtRotation` (`self.K2_GetActorLocation`) (`self.K2_GetActorLocation` _asfirst_person_character))))
      (:`then_1`
        (if (`self.SpawnProjectile`)
          (bind _returnvalue (`|SpawnActorFromClass` "/Game/FirstPersonBP/Blueprints/enemy_projectile.enemy_projectile_C" (`SceneComponent.K2_GetComponentToWorld` (`self.ProjectileSpawnLocation`)) "Undefined" "OverrideRootScale"))
          (`PrimitiveComponent.AddImpulse` (`/Game/FirstPersonBP/Blueprints/enemy_projectile.Sphere` _returnvalue) (* (`SceneComponent.GetForwardVector` (`self.CollisionMesh`)) (`self.ShootAmount`)) "None" true)
          (set `self.SpawnProjectile` false)
          (`KismetSystemLibrary.Delay` 1.0)
          (set `self.SpawnProjectile` true))))))

(event `self.CollisionMesh.OnComponentHit`
  (params (HitComponent :type "PrimitiveComponent Object Reference") (OtherActor :type "Actor Object Reference") (OtherComp :type "PrimitiveComponent Object Reference") (NormalImpulse :type "Vector Structure") (Hit :type "HitResult Structure (by ref)"))
  (bind _asenemy_turret (cast `/Game/Blueprints/enemy_turret` (`.HitActor` (`GameplayStatics.BreakHitResult` Hit))))
  (`GameplayStatics.ApplyDamage` _asenemy_turret 1.0))

(event `self.ReceiveAnyDamage`
  (params (Damage :type "Float (single-precision)") (DamageType :type "DamageType Object Reference") (InstigatedBy :type "Controller Object Reference") (DamageCauser :type "Actor Object Reference"))
  (bind _returnvalue (`self.K2_GetActorLocation`))
  (if (`self.IsAlive`)
    (bind _output_get (set `self.Health` (`KismetMathLibrary.FClamp` (- (`self.Health`) Damage) 0.0 100.0)))
    (if (<= _output_get 0.0)
      (`GameplayStatics.SpawnEmitterAtLocation` "/Game/StarterContent/Particles/P_Explosion.P_Explosion" _returnvalue)
      (`GameplayStatics.SpawnSoundAtLocation` "/Game/StarterContent/Audio/Explosion01.Explosion01" _returnvalue)
      (`DestructibleComponent.ApplyRadiusDamage` (`self.sphere_dm`) 1.0 (`SceneComponent.K2_GetComponentLocation` (`self.CollisionMesh`)) 0.0 0.0 false)
      (set `self.IsAlive` false)
      (`KismetSystemLibrary.Delay` 10.0)
      (`self.K2_DestroyActor`))))

(fn `UserConstructionScript`)